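; Solo game mode that runs a timed level of enemy waves.
; StartGame starts the level timer, HUD countdown and looping SpawnWave, which places mostly orcs, rarely ogres, at random unrepeated points into EnemiesPool.
; Player death clears enemies and bonuses and pauses timers, then respawns and resumes while lives remain.
; Timer end stops spawning and an emptied pool only prints readiness to transition; the startup and event-binding chain is disconnected from BeginPlay.
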(event EventBeginPlay)

(event EventTick
  (params (DeltaSeconds :type Float%20%28single-precision%29))
  (Development|PrintText (Utilities|Text|FormatText "Pool:{1} 
" (Utilities|Array|Length (Variables|Default|GetEnemiesPool))) true false "(R=0.000000,G=0.660000,B=1.000000,A=1.000000)" 0.0))

(fn ConstructionScript)

(fn SpawnWave
  (Utilities|Array|Clear (Variables|Default|GetFreeSpawners))
  (for (_ _array_index) (Variables|Default|GetSpawnersLocations_Enemies)
    (Utilities|Array|Add (Variables|Default|GetFreeSpawners) _array_index))
  (LocalVariables|SetL_EnemiesInWave (Math|Random|RandomIntegerinRange 3 6))
  (for _index (range 0 (- (LocalVariables|GetL_EnemiesInWave) 1))
    (LocalVariables|SetL_SpawnerIndex (Math|Random|RandomIntegerinRange 0 (- (Utilities|Array|Length (Variables|Default|GetFreeSpawners)) 1)))
    (bind _returnvalue (Game|SpawnActorfromClass "/Game/BP/EnemyPawn.EnemyPawn_C" (Math|Conversions|ToTransform(Vector) (Utilities|Array|Get(acopy) (Variables|Default|GetSpawnersLocations_Enemies) (Utilities|Array|Get(acopy) (Variables|Default|GetFreeSpawners) (LocalVariables|GetL_SpawnerIndex)))) "DontSpawnIfColliding" 0 (select (Math|Random|RandomBoolwithWeight 0.95) (Variables|Default|GetOrcTemplate) (Variables|Default|GetOgreTemplate)) 0))
    (Utilities|Array|Add (Variables|Default|GetEnemiesPool) _returnvalue)
    (Utilities|Array|RemoveIndex (Variables|Default|GetFreeSpawners) (LocalVariables|GetL_SpawnerIndex))))

(fn StartGame
  (bind _returnvalue (Utilities|Time|SetTimerbyFunctionName 0 "EndLevel" (Variables|Default|GetLevelTime)))
  (Variables|Default|SetTH_EndLevel _returnvalue)
  (Default|StartTimer (Variables|Default|GetUIRef_Gameplay) (Utilities|Time|GetTimeSeconds) (Variables|Default|GetLevelTime))
  (bind _returnvalue_2 (Utilities|Time|SetTimerbyFunctionName 0 "SpawnWave" 5.0 true))
  (Variables|Default|SetTH_SpawnWave _returnvalue_2)
  (CallFunction|SpawnWave)
  (Variables|Default|SetisTimerFinished false))

(fn EndLevel
  (Variables|Default|SetisTimerFinished true)
  (Utilities|Time|ClearandInvalidateTimerbyHandle (Variables|Default|GetTH_SpawnWave)))

(fn RemoveEnemyfromPool
  (params (Pawn :type Enemy%20Pawn%20Object%20Reference))
  (Utilities|Array|RemoveItem (Variables|Default|GetEnemiesPool) Pawn)
  (if (and (Variables|Default|GetisTimerFinished) (== (Utilities|Array|Length (Variables|Default|GetEnemiesPool)) 0))
    (Development|PrintString "ReadyToTransition!")))

(fn OnPlayerDied
  (CallFunction|ClearEnemiesPool)
  (CallFunction|ClearBonuses)
  (CallFunction|PauseTimer)
  (Utilities|Time|ClearandInvalidateTimerbyHandle (Variables|Default|GetTH_SpawnWave)))

(fn PauseTimer
  (Utilities|Time|PauseTimerbyHandle (Variables|Default|GetTH_EndLevel))
  (Default|PauseTimer (Variables|Default|GetUIRef_Gameplay) (Utilities|Time|GetTimeSeconds)))

(fn UnPauseTimer
  (Utilities|Time|UnpauseTimerbyHandle (Variables|Default|GetTH_EndLevel))
  (Default|UnpauseTimer (Variables|Default|GetUIRef_Gameplay) (Utilities|Time|GetTimeSeconds))
  (bind _returnvalue (Utilities|Time|SetTimerbyFunctionName 0 "SpawnWave" 5.0 true))
  (Variables|Default|SetTH_SpawnWave _returnvalue)
  (CallFunction|SpawnWave))

(fn ClearEnemiesPool
  (for _array_element (Variables|Default|GetEnemiesPool)
    (Actor|DestroyActor _array_element))
  (Utilities|Array|Clear (Variables|Default|GetEnemiesPool)))

(fn ClearBonuses
  (bind _outactors (Actor|GetAllActorsOfClass "/Game/BP/Bonus.Bonus_C"))
  (for _array_element _outactors
    (Default|Destroy _array_element)))

(fn OnPlayerDeathFinishedPlaying
  (params (Lifes :type Integer))
  (if (< Lifes 0)
    (Development|PrintString "RE")
    (else
      (Default|Respawn (Variables|Default|GetPlayerPawn) (Utilities|Array|Get(acopy) (Variables|Default|GetSpawnersLocations_Player)))
      (Utilities|Time|SetTimerbyFunctionName 0 "UnPauseTimer" 3.0)
      (Default|CallPlayerRespawn))))